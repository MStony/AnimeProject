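; Debug actor that lets the player change game speed from the keyboard.
; On BeginPlay it enables input from player controller 0 so the actor receives key presses directly.
; Number keys 1 through 9 run the slomo console command at matching tenth-step speeds, and 0 restores normal speed.
; Each press also prints the command on screen.
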(event `self.ReceiveBeginPlay`
  (`self.EnableInput` (`GameplayStatics.GetPlayerController` 0)))

(event `Key|One`
  (params (Key :type "Key Structure" :default "AnyKey"))
  (:`Pressed`
    (`KismetSystemLibrary.PrintString` "slomo 0.1")
    (`KismetSystemLibrary.ExecuteConsoleCommand` "slomo 0.1")))

(event `Key|Two`
  (params (Key :type "Key Structure" :default "AnyKey"))
  (:`Pressed`
    (`KismetSystemLibrary.PrintString` "slomo 0.2")
    (`KismetSystemLibrary.ExecuteConsoleCommand` "slomo 0.2")))

(event `Key|Three`
  (params (Key :type "Key Structure" :default "AnyKey"))
  (:`Pressed`
    (`KismetSystemLibrary.PrintString` "slomo 0.3")
    (`KismetSystemLibrary.ExecuteConsoleCommand` "slomo 0.3")))

(event `Key|Four`
  (params (Key :type "Key Structure" :default "AnyKey"))
  (:`Pressed`
    (`KismetSystemLibrary.PrintString` "slomo 0.4")
    (`KismetSystemLibrary.ExecuteConsoleCommand` "slomo 0.4")))

(event `Key|Five`
  (params (Key :type "Key Structure" :default "AnyKey"))
  (:`Pressed`
    (`KismetSystemLibrary.PrintString` "slomo 0.5")
    (`KismetSystemLibrary.ExecuteConsoleCommand` "slomo 0.5")))

(event `Key|Six`
  (params (Key :type "Key Structure" :default "AnyKey"))
  (:`Pressed`
    (`KismetSystemLibrary.PrintString` "slomo 0.6")
    (`KismetSystemLibrary.ExecuteConsoleCommand` "slomo 0.6")))

(event `Key|Seven`
  (params (Key :type "Key Structure" :default "AnyKey"))
  (:`Pressed`
    (`KismetSystemLibrary.PrintString` "slomo 0.7")
    (`KismetSystemLibrary.ExecuteConsoleCommand` "slomo 0.7")))

(event `Key|Eight`
  (params (Key :type "Key Structure" :default "AnyKey"))
  (:`Pressed`
    (`KismetSystemLibrary.PrintString` "slomo 0.8")
    (`KismetSystemLibrary.ExecuteConsoleCommand` "slomo 0.8")))

(event `Key|Nine`
  (params (Key :type "Key Structure" :default "AnyKey"))
  (:`Pressed`
    (`KismetSystemLibrary.PrintString` "slomo 0.9")
    (`KismetSystemLibrary.ExecuteConsoleCommand` "slomo 0.9")))

(event `Key|Zero`
  (params (Key :type "Key Structure" :default "AnyKey"))
  (:`Pressed`
    (`KismetSystemLibrary.PrintString` "slomo 1")
    (`KismetSystemLibrary.ExecuteConsoleCommand` "slomo 1")))

(fn `UserConstructionScript`)